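; Doorway actor for demo levels that plays a cutscene when a first- or third-person character enters while it is usable.
; Overlap toggles visibility on the character and plays the level sequence once until SpawnPawn re-arms it by replacing the player with a possessed ThirdPersonCharacter.
; Separate events swing the door via timeline with delayed auto-close, toggle usability, and load levels, stepping LoopInstance's index up, or down for back doors.
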(event `self.ReceiveActorBeginOverlap`
  (params (OtherActor :type "Actor Object Reference"))
  (if (`self.CanUse`)
    (bind _asfirst_person_character (cast `/Game/Demo_Content/Blueprints/MiniMap/FirstPersonCharacter` OtherActor)
      (:`then`
        (if (not (`self.End`))
          (set `self.End` true)
          (`/Game/Demo_Content/Blueprints/MiniMap/FirstPersonCharacter.Toggle Visibility` _asfirst_person_character)
          (bind (_outactor _returnvalue) (`LevelSequencePlayer.CreateLevelSequencePlayer` (`self.Cutscene`) :!label _label))
          (`MovieSceneSequencePlayer.Play` (`LevelSequenceActor.SequencePlayer` _outactor))
          (`MovieSceneSequencePlayer.Play` _returnvalue)))
      (:`CastFailed`
        (bind _asthird_person_character (cast `/Game/Demo_Content/Blueprints/ThirdPersonCharacter` OtherActor))
        (if (not (`self.End`))
          (set `self.End` true)
          (`/Game/Demo_Content/Blueprints/ThirdPersonCharacter.Toggle Visibility` _asthird_person_character)
          (goto _label))))))

(event `OpenDoor`
  (bind (_returnvalue_roll _returnvalue_pitch) (`KismetMathLibrary.BreakRotator` (`SceneComponent.K2_GetComponentRotation` (`self.Door`))))
  (set `self.HasOpen` false)
  (bind (_direction _door_move) (`Timeline|Open` :!via `PlayFromStart` :!label _label_2)
    (:`Update`
      (`SceneComponent.K2_SetWorldRotation` (`self.Door`) (`KismetMathLibrary.MakeRotator` _returnvalue_roll _returnvalue_pitch (`KismetMathLibrary.Lerp` 0.0 90.0 _door_move)) false false))
    (:`Finished`
      (`KismetSystemLibrary.Delay` 3.0)
      (if (not (`self.HasOpen`))
        (`self.Reverse`)))))

(event `Reverse`
  (set `self.HasOpen` true)
  (goto _label_2 :!via `Reverse`))

(event `SpawnPawn`
  (bind _returnvalue (`AIBlueprintHelperLibrary.SpawnAIFromClass` "/Game/Demo_Content/Blueprints/ThirdPersonCharacter.ThirdPersonCharacter_C" null (`self.SpawnLocation`)))
  (`self.K2_DestroyActor` (`GameplayStatics.GetPlayerCharacter` 0))
  (`Controller.Possess` (`GameplayStatics.GetPlayerController` 0) _returnvalue)
  (set `self.End` false))

(event `Load Level`
  (`GameplayStatics.OpenLevel` (`self.Level Name`)))

(event `Loop_Level`
  (bind _asloop_instance (cast `/Game/Demo_Content/Blueprints/Save_System/LoopInstance` (`GameplayStatics.GetGameInstance`) :!pure true))
  (bind _index (`/Game/Demo_Content/Blueprints/Save_System/LoopInstance.Index` _asloop_instance))
  (if (`self.Back_Door`)
    (bind _output_get (set `/Game/Demo_Content/Blueprints/Save_System/LoopInstance.Index` (- _index 1) _asloop_instance))
    (if (<= _output_get 0)
      (set `/Game/Demo_Content/Blueprints/Save_System/LoopInstance.Index` 0 (cast `/Game/Demo_Content/Blueprints/Save_System/LoopInstance` (`GameplayStatics.GetGameInstance`) :!pure true))
      (set `self.Level Name` "Map_Per"))
    (`self.Load Level`)
    (else
      (set `/Game/Demo_Content/Blueprints/Save_System/LoopInstance.Index` (+ _index 1) _asloop_instance)
      (`self.Load Level`))))

(event `Toggle_CanUse`
  (if (`self.CanUse`)
    (set `self.CanUse` false)
    (else
      (set `self.CanUse` true))))

(fn `UserConstructionScript`)