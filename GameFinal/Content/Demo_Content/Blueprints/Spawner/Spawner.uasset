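; Spawner that populates a looping puzzle room on BeginPlay, choosing one of seven layouts from GameInstance loop index modulo 8 plus a Mod offset.
; Layouts spawn colored cubes, a replacement floor, or stairs, platforms, buttons and possession pieces, often toggling and linking FrontDoor.
; On loop five exactly, it swaps the player's pawn for a possessed cube and spawns a ThirdPersonCharacter as AI.
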(event `self.ReceiveBeginPlay`
  (bind _output_get (set `self.Index` (+ (`self.Mod`) (mod (`/Game/Demo_Content/Blueprints/Save_System/LoopInstance.Index` (cast `/Game/Demo_Content/Blueprints/Save_System/LoopInstance` (`GameplayStatics.GetGameInstance`) :!pure true)) 8))))
  (switch `int` _output_get
    (:`1`
      (`self.One`))
    (:`2`
      (`self.Two`))
    (:`3`
      (`self.Three`))
    (:`4`
      (`self.Four`))
    (:`5`
      (`self.Five`))
    (:`6`
      (`self.Six`))
    (:`7`
      (`self.Seven`))))

(event `One`
  (for _index (range 4)
    (bind _returnvalue (`|SpawnActorFromClass` "/Game/Demo_Content/Blueprints/Spawner/Assets/ColorCube.ColorCube_C" (`KismetMathLibrary.MakeTransform` (+ (`self.K2_GetActorLocation`) (`|GetArrayItem` (`self.Locations`) _index))) "Undefined" "OverrideRootScale" null null))
    (`PrimitiveComponent.SetMaterial` (`/Game/Demo_Content/Blueprints/Spawner/Assets/ColorCube.Cube` _returnvalue) 0 (`|GetArrayItem` (`self.Materials`) _index))))

(event `Two`
  (bind _front_door (`self.Front_Door`))
  (`self.Spawn_Stairs`)
  (bind _returnvalue (`|SpawnActorFromClass` "/Game/Demo_Content/Blueprints/Buttons/Button.Button_C" (`KismetMathLibrary.MakeTransform` (+ (`self.K2_GetActorLocation`) (1000.0 700.0 450.0)) (struct :`Yaw` 90.0)) "Undefined" "OverrideRootScale" null null))
  (`/Engine/EditorBlueprintResources/StandardMacros.IsValid` _front_door
    (:`Is Valid`
      (bind _output_get (set `/Game/Demo_Content/Blueprints/Buttons/Button.Door` _front_door _returnvalue))
      (`/Game/Demo_Content/Blueprints/DoorWay.Toggle_CanUse` _output_get))))

(event `Three`
  (bind _floor (`self.Floor`))
  (bind (_returnvalue_location _returnvalue_rotation) (`KismetMathLibrary.BreakTransform` (`self.GetTransform` _floor)))
  (`/Engine/EditorBlueprintResources/StandardMacros.IsValid` _floor
    (:`Is Valid`
      (`|SpawnActorFromClass` "/Game/Demo_Content/Blueprints/Spawner/Assets/FloorColored.FloorColored_C" (`KismetMathLibrary.MakeTransform` _returnvalue_location _returnvalue_rotation) "Undefined" "OverrideRootScale" null null)
      (`KismetSystemLibrary.Delay` 0.2)
      (`self.K2_DestroyActor` (`self.Floor`)))))

(event `Four`
  (bind _front_door (`self.Front_Door`))
  (`self.Spawn_Stairs`)
  (bind _returnvalue (`|SpawnActorFromClass` "/Game/Demo_Content/Blueprints/Buttons/Button.Button_C" (`KismetMathLibrary.MakeTransform` (+ (`self.K2_GetActorLocation`) (1000.0 -700.0 450.0))) "Undefined" "OverrideRootScale" null null))
  (`/Engine/EditorBlueprintResources/StandardMacros.IsValid` _front_door
    (:`Is Valid`
      (bind _output_get (set `/Game/Demo_Content/Blueprints/Buttons/Button.Door` _front_door _returnvalue))
      (`/Game/Demo_Content/Blueprints/DoorWay.Toggle_CanUse` _output_get)
      (`|SpawnActorFromClass` "/Game/Demo_Content/Blueprints/Spawner/Assets/Platform.Platform_C" (`KismetMathLibrary.MakeTransform` (+ (`self.K2_GetActorLocation`) (1025.0 -750.0 380.0)) (struct) (2.5 4.0 1.0)) "Undefined" "OverrideRootScale" null null)
      (bind _returnvalue_2 (`|SpawnActorFromClass` "/Game/Demo_Content/Blueprints/Platform/Platform_Move.Platform_Move_C" (`KismetMathLibrary.MakeTransform` (+ (`self.K2_GetActorLocation`) (1025.0 400.0 380.0)) (struct) (2.0 2.0 1.0)) "Undefined" "OverrideRootScale" null null))
      (set `/Game/Demo_Content/Blueprints/Platform/Platform_Move.Location` (+ (`self.K2_GetActorLocation`) (1025.0 -400.0 380.0)) _returnvalue_2))))

(event `Five`
  (`self.Spawn_Stairs`)
  (if (== (`/Game/Demo_Content/Blueprints/Save_System/LoopInstance.Index` (cast `/Game/Demo_Content/Blueprints/Save_System/LoopInstance` (`GameplayStatics.GetGameInstance`) :!pure true)) 5)
    (`KismetSystemLibrary.Delay` 0.1)
    (`self.Spawn_Cube`)
    (`AIBlueprintHelperLibrary.SpawnAIFromClass` "/Game/Demo_Content/Blueprints/ThirdPersonCharacter.ThirdPersonCharacter_C" null (+ (`self.K2_GetActorLocation`) (920.0 700.0 50.0)) (struct :`Yaw` 270.0))))

(event `Seven`
  (bind (_returnvalue_x _returnvalue_y _returnvalue_z) (`KismetMathLibrary.BreakVector` (`self.K2_GetActorLocation`)))
  (bind _front_door (`self.Front_Door`))
  (`/Engine/EditorBlueprintResources/StandardMacros.IsValid` _front_door
    (:`Is Valid`
      (`/Game/Demo_Content/Blueprints/DoorWay.Toggle_CanUse` _front_door))
    (:`Is Not Valid`
      _))
  (bind _returnvalue (`|SpawnActorFromClass` "/Game/Demo_Content/Blueprints/Buttons/Button.Button_C" (`KismetMathLibrary.MakeTransform` (`KismetMathLibrary.MakeVector` _returnvalue_x _returnvalue_y (+ _returnvalue_z 50.0)) (struct :`Yaw` 90.0)) "Undefined" "OverrideRootScale" null null))
  (set `/Game/Demo_Content/Blueprints/Buttons/Button.Door_Button` false _returnvalue))

(event `Six`
  (bind _front_door (`self.Front_Door`))
  (`self.Spawn_Stairs`)
  (bind _returnvalue (`|SpawnActorFromClass` "/Game/Demo_Content/Blueprints/Spawner/Possesion_Cube/Possesion_Platform.Possesion_Platform_C" (`KismetMathLibrary.MakeTransform` (+ (`self.K2_GetActorLocation`) (1000.0 -700.0 425.0))) "Undefined" "OverrideRootScale" null null))
  (`/Engine/EditorBlueprintResources/StandardMacros.IsValid` _front_door
    (:`Is Valid`
      (bind _output_get (set `/Game/Demo_Content/Blueprints/Spawner/Possesion_Cube/Possesion_Platform.Door` _front_door _returnvalue))
      (`/Game/Demo_Content/Blueprints/DoorWay.Toggle_CanUse` _output_get)
      (`|SpawnActorFromClass` "/Game/Demo_Content/Blueprints/Spawner/Assets/Platform.Platform_C" (`KismetMathLibrary.MakeTransform` (+ (`self.K2_GetActorLocation`) (1025.0 -750.0 380.0)) (struct) (2.5 4.0 1.0)) "Undefined" "OverrideRootScale" null null)
      (bind _returnvalue_2 (`|SpawnActorFromClass` "/Game/Demo_Content/Blueprints/Platform/Platform_Move.Platform_Move_C" (`KismetMathLibrary.MakeTransform` (+ (`self.K2_GetActorLocation`) (1025.0 400.0 380.0)) (struct) (2.0 2.0 1.0)) "Undefined" "OverrideRootScale" null null))
      (set `/Game/Demo_Content/Blueprints/Platform/Platform_Move.Location` (+ (`self.K2_GetActorLocation`) (1025.0 -400.0 380.0)) _returnvalue_2)
      (`AIBlueprintHelperLibrary.SpawnAIFromClass` "/Game/Demo_Content/Blueprints/Spawner/Possesion_Cube/Possesion_Cube.Possesion_Cube_C" null (+ (`self.K2_GetActorLocation`) (920.0 700.0 50.0)) (struct :`Yaw` 270.0)))))

(fn `Spawn_Cube`
  (bind _output_get (set `self.TempLocation` (`self.K2_GetActorLocation` (`GameplayStatics.GetPlayerCharacter` 0))))
  (`self.K2_DestroyActor` (`GameplayStatics.GetPlayerPawn` 0))
  (bind _returnvalue (`AIBlueprintHelperLibrary.SpawnAIFromClass` "/Game/Demo_Content/Blueprints/Spawner/Possesion_Cube/Possesion_Cube.Possesion_Cube_C" null _output_get))
  (`Controller.Possess` (`GameplayStatics.GetPlayerController` 0) _returnvalue))

(fn `Spawn_Stairs`
  (`|SpawnActorFromClass` "/Game/Demo_Content/Blueprints/Spawner/Assets/Stairs.Stairs_C" (`KismetMathLibrary.MakeTransform` (+ (`self.K2_GetActorLocation`) (300.0 530.0 40.0)) (struct) (2.0 2.0 2.0)) "Undefined" "OverrideRootScale" null null)
  (`|SpawnActorFromClass` "/Game/Demo_Content/Blueprints/Spawner/Assets/Platform.Platform_C" (`KismetMathLibrary.MakeTransform` (+ (`self.K2_GetActorLocation`) (1025.0 750.0 380.0)) (struct) (2.5 4.0 1.0)) "Undefined" "OverrideRootScale" null null))

(fn `UserConstructionScript`)