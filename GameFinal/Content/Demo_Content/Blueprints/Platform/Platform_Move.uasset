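; Moving platform that slides along the world Y axis when the ThirdPersonCharacter or a Possesion_Cube overlaps it.
; On overlap it saves its current location and plays the Move timeline from the start, lerping only Y toward the stored Location.
; When the timeline finishes, the saved start point becomes the new Location, so the next overlap sends the platform back the other way.
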(event `self.ReceiveActorBeginOverlap`
  (params (OtherActor :type "Actor Object Reference"))
  (bind (_location_x _location_y) (`KismetMathLibrary.BreakVector` (`self.Location`)))
  (bind (_currentlocation_x _currentlocation_y _currentlocation_z) (`KismetMathLibrary.BreakVector` (`self.CurrentLocation`)))
  (cast `/Game/Demo_Content/Blueprints/ThirdPersonCharacter` OtherActor
    (:`then`
      _)
    (:`CastFailed`
      (cast `/Game/Demo_Content/Blueprints/Spawner/Possesion_Cube/Possesion_Cube` OtherActor)))
  (set `self.CurrentLocation` (`self.K2_GetActorLocation`))
  (bind (_direction _alpha) (`Timeline|Move` :!via `PlayFromStart`)
    (:`Update`
      (`self.K2_SetActorLocation` (`KismetMathLibrary.MakeVector` _currentlocation_x (`KismetMathLibrary.Lerp` _currentlocation_y _location_y _alpha) _currentlocation_z)))
    (:`Finished`
      (set `self.Location` (`self.CurrentLocation`)))))

(fn `UserConstructionScript`)