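; Wall button Blueprint that, when pressed, either toggles whether its linked door can be used or loads the Map_Per level.
; Press_Button swaps the button mesh to a dark red material and waits one second before acting.
; The DoorButton flag selects the door branch, which also restores the red material through TurnOn; the level-load branch does not.
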(event `Press_Button`
  (`PrimitiveComponent.SetMaterial` (`self.Button`) 0 "/Game/Demo_Content/Materials/Button_DarkRed.Button_DarkRed")
  (`KismetSystemLibrary.Delay` 1.0)
  (if (`self.Door_Button`)
    (`/Game/Demo_Content/Blueprints/DoorWay.Toggle_CanUse` (`self.Door`))
    (`self.Turn On`)
    (else
      (`GameplayStatics.OpenLevel` "Map_Per"))))

(event `Turn On`
  (`PrimitiveComponent.SetMaterial` (`self.Button`) 0 "/Game/Demo_Content/Materials/Button_Red.Button_Red"))

(fn `UserConstructionScript`)