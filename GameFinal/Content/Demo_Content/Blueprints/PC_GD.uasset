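; Player controller for a possession mechanic that moves control between ThirdPersonCharacter and Possesion_Cube pawns.
; Interaction traces forward from the player character on the Camera channel, records previous and new characters, and calls PossesMe on a hit pawn.
; The same input then traces on the Visibility channel to press any Button hit.
; Key 1 swaps the two stored characters and possesses the earlier one.
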(event `InputAction|Interaction`
  (params (Key :type "Key Structure"))
  (:`Pressed`
    (`self.SearchForPawn`)))

(event `Key|One`
  (params (Key :type "Key Structure"))
  (bind _newcharacter (`self.NewCharacter`))
  (:`Pressed`
    (if (and (`KismetSystemLibrary.IsValid` (`self.Previous Character`)) (`KismetSystemLibrary.IsValid` (`self.NewCharacter`)))
      (set `self.CharacterMem` (`self.NewCharacter`))
      (set `self.NewCharacter` (`self.Previous Character`))
      (set `self.Previous Character` (`self.CharacterMem`))
      (`|ExecutionSequence`
        (:`then_0`
          (bind _aspossesion_cube (cast `/Game/Demo_Content/Blueprints/Spawner/Possesion_Cube/Possesion_Cube` _newcharacter))
          (`/Game/Demo_Content/Blueprints/Spawner/Possesion_Cube/Possesion_Cube.Posses_Me` _aspossesion_cube))
        (:`then_1`
          (bind _asthird_person_character (cast `/Game/Demo_Content/Blueprints/ThirdPersonCharacter` _newcharacter))
          (`/Game/Demo_Content/Blueprints/ThirdPersonCharacter.Posses_Me` _asthird_person_character))))))

(fn `SearchForButton`
  (bind _returnvalue (`GameplayStatics.GetPlayerCharacter` 0))
  (bind _returnvalue_2 (`self.K2_GetActorLocation` _returnvalue))
  (bind _outhit (`KismetSystemLibrary.LineTraceSingle` _returnvalue_2 (+ _returnvalue_2 (* (`self.GetActorForwardVector` _returnvalue) 400.0)) "TraceTypeQuery1" false (`|MakeArray` _returnvalue :!type "Actor Object Reference")))
  (bind _asbutton (cast `/Game/Demo_Content/Blueprints/Buttons/Button` (`.HitActor` (`GameplayStatics.BreakHitResult` _outhit))))
  (`/Game/Demo_Content/Blueprints/Buttons/Button.Press_Button` _asbutton))

(fn `SearchForPawn`
  (bind _returnvalue (`GameplayStatics.GetPlayerCharacter` 0))
  (bind _returnvalue_2 (`self.K2_GetActorLocation` _returnvalue))
  (set `self.Previous Character` _returnvalue)
  (bind _outhit (`KismetSystemLibrary.LineTraceSingle` _returnvalue_2 (+ _returnvalue_2 (* (`self.GetActorForwardVector` _returnvalue) 400.0)) "TraceTypeQuery2" false (`|MakeArray` _returnvalue :!type "Actor Object Reference")))
  (`|ExecutionSequence`
    (:`then_0`
      (bind (_bblockinghit _binitialoverlap _time _distance _location _impactpoint _normal _impactnormal _physmat _hitactor) (`GameplayStatics.BreakHitResult` _outhit))
      (bind _aspossesion_cube (cast `/Game/Demo_Content/Blueprints/Spawner/Possesion_Cube/Possesion_Cube` _hitactor))
      (set `self.NewCharacter` _aspossesion_cube)
      (`/Game/Demo_Content/Blueprints/Spawner/Possesion_Cube/Possesion_Cube.Posses_Me` _aspossesion_cube))
    (:`then_1`
      (bind _asthird_person_character (cast `/Game/Demo_Content/Blueprints/ThirdPersonCharacter` _hitactor))
      (set `self.NewCharacter` _asthird_person_character)
      (`/Game/Demo_Content/Blueprints/ThirdPersonCharacter.Posses_Me` _asthird_person_character))
    (:`then_2`
      (`self.SearchForButton`))))

(fn `UserConstructionScript`)